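; BP_Base_Mag is the base magazine attachment in the FPS controller, with separate first-person and third-person meshes.
; BeginPlay hides the mag_02 bone on the third-person mesh, and PlayReloadAnimation plays a tactical reload animation on the first-person mesh.
; OnRepAttachment passes BulletsPerMag to the owner through SetMagAmmoMessage.
; Accessor functions return each mesh, and DestroyFPPComponent removes the first-person one.
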(event Custom|PlayReloadAnimation
  (Components|Animation|PlayAnimation (Variables|Default|GetFPPMesh) (Variables|Default|GetMagTacticalReload) false))

(event EventBeginPlay
  (|CallParentFunction)
  (Components|SkinnedMesh|HideBonebyName (Variables|Default|GetTPPMesh) "mag_02" "PBO_None"))

(event Collision|EventActorBeginOverlap
  (params (OtherActor :type Actor%20Object%20Reference))
  (|CallParentFunction OtherActor) ; This node is disabled and will not be called.\nDrag off pins to build functionality.
)

(event EventTick
  (params (DeltaSeconds :type Float%20%28single-precision%29))
  (|CallParentFunction DeltaSeconds) ; This node is disabled and will not be called.\nDrag off pins to build functionality.
)

(event EventOnRepAttachment
  (Class|BIWeapon|SetMagAmmo(Message) (Components|GetOwner) (Variables|Default|GetBulletsPerMag)))

(fn ConstructionScript
  (|CallParentFunction))

(fn GetFPPMesh
  (return (Variables|Default|GetFPPMesh)))

(fn GetTPPMesh
  (return (Variables|Default|GetTPPMesh)))

(fn DestroyFPPComponent
  (Components|DestroyComponent (Variables|Default|GetFPPMesh)))