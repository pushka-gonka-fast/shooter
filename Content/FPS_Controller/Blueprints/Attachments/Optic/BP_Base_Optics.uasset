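; BP_Base_Optics is the base weapon optic attachment for the FPS controller, setting the aiming field of view of whatever owns it.
; When the attachment replication event fires, it passes its AimFOV to the owner through SetAimFOVMessage.
; It exposes separate first-person and third-person meshes through getters, and can destroy the first-person mesh component on its own.
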(event EventOnRepAttachment1
  (Class|BIWeapon|SetAimFOV(Message) (Components|GetOwner) (Variables|Default|GetAimFOV)))

(fn ConstructionScript
  (|CallParentFunction))

(fn GetFPPMesh
  (return (Variables|Default|GetFPPMesh)))

(fn GetTPPMesh
  (return (Variables|Default|GetTPPMesh)))

(fn DestroyFPPComponent
  (Components|DestroyComponent (Variables|Default|GetFPPMesh)))