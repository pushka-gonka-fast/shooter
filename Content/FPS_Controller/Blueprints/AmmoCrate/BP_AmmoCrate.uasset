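; BP_AmmoCrate is an ammo pickup crate that refills a player's ammo and adds lethal ammo on overlap.
; The inner Sphere calls the overlapping actor's AC_InventorySystem and plays a 2D reload sound, all on authority only.
; A separate WidgetSphere shows and hides a widget message for locally controlled players.
; A delayed BeginPlay check shows the message for characters already inside that sphere.
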(event OnComponentBeginOverlap(Sphere)
  (params (OverlappedComponent :type Primitive%20Component%20Object%20Reference) (OtherActor :type Actor%20Object%20Reference) (OtherComp :type Primitive%20Component%20Object%20Reference) (OtherBodyIndex :type Integer) (bFromSweep :type Boolean) (SweepResult :type Hit%20Result%20Structure%20%28by%20ref%29))
  (bind _returnvalue (Actor|GetComponentbyClass OtherActor "/Game/FPS_Controller/Blueprints/Components/AC_InventorySystem.AC_InventorySystem_C"))
  ;[0 0 0] On Overlap Trigger Sphere
  (Variables|Default|SetbUsed false)
  (Networking|SwitchHasAuthority
    (:Authority
      (Default|RefillAmmo _returnvalue)
      (Default|AddLethalAmmo _returnvalue)
      (Audio|PlaySound2D "/Game/FPS_Controller/Audio/Rifle/Mag/SC_AR_Mag30_In.SC_AR_Mag30_In" 1.0 1.0 0.0 0 0))))

(event OnComponentBeginOverlap(WidgetSphere)
  (params (OverlappedComponent :type Primitive%20Component%20Object%20Reference) (OtherActor :type Actor%20Object%20Reference) (OtherComp :type Primitive%20Component%20Object%20Reference) (OtherBodyIndex :type Integer) (bFromSweep :type Boolean) (SweepResult :type Hit%20Result%20Structure%20%28by%20ref%29))
  ;[0 0 0] On Overlap Widget Trigger Sphere
  (if (Pawn|IsLocallyControlled (Variables|/Script/Engine.Actor|GetInstigator OtherActor))
    (Class|BIUI|ShowWidget(Message) (UserInterface|GetUserWidgetObject (Variables|Default|GetWidget)))))

(event OnComponentEndOverlap(WidgetSphere)
  (params (OverlappedComponent :type Primitive%20Component%20Object%20Reference) (OtherActor :type Actor%20Object%20Reference) (OtherComp :type Primitive%20Component%20Object%20Reference) (OtherBodyIndex :type Integer))
  ;[0 0 0] End Overlap Widget Trigger Sphere
  (if (Pawn|IsLocallyControlled (Variables|/Script/Engine.Actor|GetInstigator OtherActor))
    (Class|BIUI|HideWidget(Message) (UserInterface|GetUserWidgetObject (Variables|Default|GetWidget)))))

(event EventBeginPlay
  ;[0 0 0] Begin Play
  (Utilities|FlowControl|Delay 1.5)
  (for _array_element (Collision|GetOverlappingActors (Variables|Default|GetWidgetSphere) "/Script/Engine.Character" :!class /Script/Engine.PrimitiveComponent)
    (if (Pawn|IsLocallyControlled (Variables|/Script/Engine.Actor|GetInstigator _array_element))
      (Class|BIUI|ShowWidget(Message) (UserInterface|GetUserWidgetObject (Variables|Default|GetWidget))))))

(fn ConstructionScript)