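; BP_GM is the FPS controller's game mode, handling HUD start-up and providing random spawn locations.
; On HUD initialization it calls SpawnMessage on player controller 0.
; GetRandomPlayerStart returns the transform of a randomly chosen PlayerStart in the level.
; The default pawn class override only defers to the parent, and a loadout selection call through AC_UI_Manager is left disconnected.
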(event EventInitializeHUDforPlayer
  (params (NewPlayer :type Player%20Controller%20Object%20Reference))
  ;[0 0 0] Load the widget
  (Class|BIPlayerController|Spawn(Message) (Game|GetPlayerController 0)))

(fn ConstructionScript)

(fn GetDefaultPawnClassforController
  (params (InController :type Controller%20Object%20Reference))
  (bind _returnvalue (|CallParentFunction InController))
  (return _returnvalue))

(fn GetRandomPlayerStart
  (bind _outactors (Actor|GetAllActorsOfClass "/Script/Engine.PlayerStart"))
  (return (Transformation|GetActorTransform (Utilities|Array|Get(acopy) _outactors (Math|Random|RandomIntegerinRange 0 (Utilities|Array|LastIndex _outactors))))))